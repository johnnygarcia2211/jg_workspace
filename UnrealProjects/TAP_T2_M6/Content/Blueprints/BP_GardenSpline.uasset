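; Procedural garden actor that builds a fenced vegetable plot on the landscape in its Construction Script.
; Pins the Path spline's ends to the boundary spline and sets material variation through MPC_Garden.
; Places seeded random fence meshes along the boundary, leaving openings at both path ends.
; MakeGrid supplies planting points and crop types, optionally overridden per cell, for instanced cabbage, corn and pumpkins, line-traced onto the landscape like the fences.
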(event EventBeginPlay)

(event Collision|EventActorBeginOverlap
  (params (OtherActor :type Actor%20Object%20Reference)))

(event EventTick
  (params (DeltaSeconds :type Float%20%28single-precision%29)))

(fn ConstructionScript
  (bind _spline (Variables|Default|GetSpline))
  (bind _path (Variables|Default|GetPath))
  (bind _transform (Variables|Vegetables|GetTransform))
  (bind _path_size (Variables|Path|GetPath%20Size))
  (bind _spline_2 (Variables|Default|GetSpline))
  (bind _path_2 (Variables|Default|GetPath))
  (bind _useshortfence (Variables|Fence|GetuseShortFence))
  (bind _fences01_ism (Variables|Default|GetFenceS01_ISM))
  (bind _fencel01_ism (Variables|Default|GetFenceL01_ISM))
  (bind _returnvalue (Spline|GetNumberOfSplinePoints _path_2))
  (bind _returnvalue_2 (Spline|GetNumberOfSplinePoints _spline))
  (bind _returnvalue_3 (select _useshortfence _fences01_ism _fencel01_ism))
  (bind _returnvalue_4 (- _returnvalue 1))
  (bind _staticmesh (Variables|/Script/Engine.StaticMeshComponent|GetStaticMesh _returnvalue_3))
  (bind _returnvalue_5 (StaticMesh|GetBoundingBox _staticmesh))
  ;[1 1 1] Materials
  (Rendering|Material|SetScalarParameterValue "/Game/Data/Collections/MPC_Garden.MPC_Garden" "VegetablesVariance" (Variables|Vegetables|GetVegetableMaterialVariation) :!class /Script/Engine.KismetMaterialLibrary)
  (Rendering|Material|SetScalarParameterValue "/Game/Data/Collections/MPC_Garden.MPC_Garden" "FenceVariance" (Variables|Fence|GetFenceMaterialVariation) :!class /Script/Engine.KismetMaterialLibrary)
  (Utilities|FlowControl|Sequence
    (:then_0
      ;[1 1 1] Path
      (Spline|SetLocationatSplinePoint _path 0 (Class|SplineComponent|GetLocationatSplineInputKey _spline (* (Variables|Path|GetEntranceU) _returnvalue_2) "Local") "Local" true)
      (Spline|SetLocationatSplinePoint _path (- (Spline|GetNumberOfSplinePoints _path) 1) (Class|SplineComponent|GetLocationatSplineInputKey _spline (* (Variables|Path|GetExitU) _returnvalue_2) "Local") "Local" true))
    (:then_1
      (if (Variables|Fence|GetplaceFence)
        ;[1 1 1] Fences
        (bind _output_get (Variables|Fence|SetFenceSpacing (.X (Math|Vector|BreakVector (- (.max _returnvalue_5) (.min _returnvalue_5))))))
        (for _index (range 0 (Math|Float|Floor (/ (Spline|GetSplineLength _spline_2) _output_get)))
          (Variables|Fence|SetFenceIndex _index)
          (if (and (> (Math|Vector2D|Vector2DLength (Math|Vector2D|MakeVector2D (.x (- (Spline|GetLocationatSplinePoint _path_2 0 "World") (Spline|GetLocationatDistanceAlongSpline _spline_2 (* _index (+ _output_get (* (Variables|Fence|GetFenceGap) (Math|Random|RandomFloatinRangefromStream (Math|Random|MakeRandomStream (* (Variables|Fence|GetFenceIndex) (Variables|Fence|GetFenceSeed))) 0.0 1.0)))) "World"))) (.y (- (Spline|GetLocationatSplinePoint _path_2 0 "World") (Spline|GetLocationatDistanceAlongSpline _spline_2 (* _index (+ _output_get (* (Variables|Fence|GetFenceGap) (Math|Random|RandomFloatinRangefromStream (Math|Random|MakeRandomStream (* (Variables|Fence|GetFenceIndex) (Variables|Fence|GetFenceSeed))) 0.0 1.0)))) "World"))))) (* _path_size (.y (Spline|GetScaleatSplinePoint _path_2 0)))) (> (Math|Vector2D|Vector2DLength (Math|Vector2D|MakeVector2D (.x (- (Spline|GetLocationatSplinePoint _path_2 _returnvalue_4 "World") (Spline|GetLocationatDistanceAlongSpline _spline_2 (* _index (+ _output_get (* (Variables|Fence|GetFenceGap) (Math|Random|RandomFloatinRangefromStream (Math|Random|MakeRandomStream (* (Variables|Fence|GetFenceIndex) (Variables|Fence|GetFenceSeed))) 0.0 1.0)))) "World"))) (.y (- (Spline|GetLocationatSplinePoint _path_2 _returnvalue_4 "World") (Spline|GetLocationatDistanceAlongSpline _spline_2 (* _index (+ _output_get (* (Variables|Fence|GetFenceGap) (Math|Random|RandomFloatinRangefromStream (Math|Random|MakeRandomStream (* (Variables|Fence|GetFenceIndex) (Variables|Fence|GetFenceSeed))) 0.0 1.0)))) "World"))))) (* _path_size (.y (Spline|GetScaleatSplinePoint _path_2 _returnvalue_4)))))
            (bind (_outhit _returnvalue_6) (Collision|LineTraceByChannel (Spline|GetLocationatDistanceAlongSpline _spline_2 (* _index (+ _output_get (* (Variables|Fence|GetFenceGap) (Math|Random|RandomFloatinRangefromStream (Math|Random|MakeRandomStream (* (Variables|Fence|GetFenceIndex) (Variables|Fence|GetFenceSeed))) 0.0 1.0)))) "World") (+ (Spline|GetLocationatDistanceAlongSpline _spline_2 (* _index (+ _output_get (* (Variables|Fence|GetFenceGap) (Math|Random|RandomFloatinRangefromStream (Math|Random|MakeRandomStream (* (Variables|Fence|GetFenceIndex) (Variables|Fence|GetFenceSeed))) 0.0 1.0)))) "World") "0.000000,0.000000,-1000.000000") "TraceTypeQuery1" false 0 (Variables|Debug|GetDraw%20Debug%20Type)))
            (if (and _returnvalue_6 (== (.HitActor (Collision|BreakHitResult _outhit)) (Variables|System|GetLandscape)))
              (Components|InstancedStaticMesh|AddInstance (select (Variables|Fence|GetuseShortFence) (Utilities|Select :Index (Math|Random|RandomIntegerinRangefromStream (Math|Random|MakeRandomStream (* (Variables|Fence|GetFenceIndex) (Variables|Fence|GetFenceSeed))) 0 2) :Option%200 (Variables|Default|GetFenceS01_ISM) :Option%201 (Variables|Default|GetFenceS02_ISM) :Option%202 (Variables|Default|GetFenceS03_ISM)) (Utilities|Select :Index (Math|Random|RandomIntegerinRangefromStream (Math|Random|MakeRandomStream (* (Variables|Fence|GetFenceIndex) (Variables|Fence|GetFenceSeed))) 0 3) :Option%200 (Variables|Default|GetFenceL01_ISM) :Option%201 (Variables|Default|GetFenceL02_ISM) :Option%202 (Variables|Default|GetFenceL03_ISM) :Option%203 (Variables|Default|GetFenceL04_ISM))) (Math|Transform|MakeTransform (Math|Vector|MakeVector (.X (Math|Vector|BreakVector (.Location (Collision|BreakHitResult _outhit)))) (.Y (Math|Vector|BreakVector (.Location (Collision|BreakHitResult _outhit)))) (+ (.Z (Math|Vector|BreakVector (.Location (Collision|BreakHitResult _outhit)))) (Math|Random|RandomFloatinRangefromStream (Math|Random|MakeRandomStream (* (Variables|Fence|GetFenceIndex) (Variables|Fence|GetFenceSeed))) 0.0 (CallFunction|NegateFloat (Variables|Fence|GetFenceZOffset))))) (Math|Rotator|MakeRotfromX (Spline|GetTangentatDistanceAlongSpline _spline_2 (* _index (+ _output_get (* (Variables|Fence|GetFenceGap) (Math|Random|RandomFloatinRangefromStream (Math|Random|MakeRandomStream (* (Variables|Fence|GetFenceIndex) (Variables|Fence|GetFenceSeed))) 0.0 1.0)))) "Local")) "1.000000,1.000000,1.000000") true))))))
    (:then_2
      ;[1 1 1] Planting Loop
      (if (Variables|Vegetables|GetplantVegetables)
        (bind (_pos _veggies) (CallFunction|MakeGrid (Variables|Default|GetPath) (Variables|Default|GetSpline) (Variables|System|GetSystemSeed) (Variables|System|GetGridSpacing) (Variables|System|GetGridPadding) (Variables|Path|GetPath%20Size) (Variables|System|GetBorderPadding) (Variables|System|GetGrid%20Rotation%20Angle) (Variables|Vegetables|GetrandomRows) (Variables|Vegetables|GetsinglePlantGarden) (Variables|Vegetables|GetSingleVegetable)))
        (Utilities|Array|Resize (Variables|Vegetables|GetVegetableTypes) (Utilities|Array|Length _pos))
        (Utilities|Array|Clear _transform)
        (for (_array_element _array_index) _pos
          (Variables|Vegetables|SetCurrentLocation (Math|Vector|MakeVector (.x _array_element) (.y _array_element) (.z (Transformation|GetActorLocation))))
          (Variables|System|SetCurrentIndex _array_index)
          (Utilities|FlowControl|Sequence
            (:then_0
              (if (Variables|Vegetables|GetManualOverride)
                (Utilities|Array|SetArrayElem _veggies (Variables|System|GetCurrentIndex) (Utilities|Array|Get(acopy) (Variables|Vegetables|GetVegetableTypes) (Variables|System|GetCurrentIndex)))
                (Variables|Vegetables|SetCurrentVegetable (Utilities|Array|Get(acopy) (Variables|Vegetables|GetVegetableTypes) (Variables|System|GetCurrentIndex)))
                (else
                  (Variables|Vegetables|SetCurrentVegetable (Utilities|Array|Get(acopy) _veggies (Variables|System|GetCurrentIndex)))
                  (Utilities|Array|SetArrayElem (Variables|Vegetables|GetVegetableTypes) (Variables|System|GetCurrentIndex) (Utilities|Array|Get(acopy) _veggies (Variables|System|GetCurrentIndex))))))
            (:then_1
              ;[1 1 1] Plant Instancing
              (Utilities|Array|AddUnique (Variables|Vegetables|GetTransform) (Math|Transform|MakeTransform (Math|Vector|MakeVector (.x (- (Variables|Vegetables|GetHitLocation) (Transformation|GetActorLocation))) (.y (- (Variables|Vegetables|GetHitLocation) (Transformation|GetActorLocation))) (+ (.z (- (Variables|Vegetables|GetHitLocation) (Transformation|GetActorLocation))) 3e+02)) "0, 0, 0" "1.000000,1.000000,1.000000"))
              (bind (_outhit_2 _returnvalue_7) (Collision|LineTraceByChannel (+ (Variables|Vegetables|GetCurrentLocation) "0.000000,0.000000,400.000000") (+ (Variables|Vegetables|GetCurrentLocation) "0.000000,0.000000,-1000.000000") "TraceTypeQuery1" false 0 (Variables|Debug|GetDraw%20Debug%20Type)))
              (bind _output_get_2 (Variables|Vegetables|SetHitLocation (.Location (Collision|BreakHitResult _outhit_2))))
              (if (and _returnvalue_7 (== (.HitActor (Collision|BreakHitResult _outhit_2)) (Variables|System|GetLandscape)))
                (Components|InstancedStaticMesh|AddInstance (Utilities|Select :Index (Variables|Vegetables|GetCurrentVegetable) :NewEnumerator0 (Variables|Default|GetCabbage_ISM) :NewEnumerator1 (Variables|Default|GetCorn_ISM) :NewEnumerator2 (Variables|Default|GetPumpkin_ISM)) (Math|Transform|MakeTransform _output_get_2 (Math|Rotator|MakeRotator 0.0 0.0 (+ (.Pitch (Math|Rotator|BreakRotator (.rotation (Utilities|Array|Get(acopy) (Variables|Vegetables|GetTransform) (Variables|System|GetCurrentIndex))))) (.yaw (Class|KismetMathLibrary|RandomRotatorfromStream (Math|Random|MakeRandomStream (* (Variables|System|GetCurrentIndex) (Variables|Vegetables|GetVegetablesSeed))) false)))) (* (.scale (Utilities|Array|Get(acopy) (Variables|Vegetables|GetTransform) (Variables|System|GetCurrentIndex))) (Math|Conversions|ToVector(Float) (Math|Float|Lerp 0.8 1.2 (Math|Random|RandomFloatfromStream (Math|Random|MakeRandomStream (* (Variables|System|GetCurrentIndex) (Variables|Vegetables|GetVegetablesSeed)))))))) true)))))
        (Utilities|Array|RemoveIndex _transform)))))