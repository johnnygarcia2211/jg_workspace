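; Blueprint function library that generates vegetable planting layouts for a garden outlined by a spline.
; MakeGrid builds a rotated grid over the spline's padded bounds from GetSplineBounds2D, at zero height.
; It keeps points inside the outline, using a cross/dot side test, that clear the border padding and the scale-dependent path spline width.
; It returns positions with cabbage, corn or pumpkin picked by seed per row or point, or one override vegetable.
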(fn MakeGrid
  (params (Path :type Spline%20Component%20Object%20Reference) (Spline :type Spline%20Component%20Object%20Reference) (Seed :type Integer) (Interval :type Float%20%28double-precision%29) (GridPadding :type Float%20%28double-precision%29) (PathSize :type Float%20%28double-precision%29) (BorderPadding :type Float%20%28double-precision%29) (GridRotationAngle :type Float%20%28double-precision%29) (bRandomRows :type Boolean) (bSinglePlantGarden :type Boolean) (OverrideVeggie :type EVegetables%20Enum :default "NewEnumerator0"))
  (bind _vegetables (LocalVariables|GetVegetables))
  (bind _max (LocalVariables|GetMax))
  (bind _positions (LocalVariables|GetPositions))
  (bind _returnvalue (Math|Float|Clamp(Float) Interval 2.0 _max))
  (bind _returnvalue_2 (Transformation|GetWorldLocation Spline))
  (bind (_x _y) (Math|Vector|BreakVector _returnvalue_2))
  ;[1 1 1] Grid Intialize
  (bind _boundscount (CallFunction|GetSplineBounds2D Spline false (Math|Float|Clamp(Float) Interval 2.0 (LocalVariables|GetMax)) GridPadding))
  (LocalVariables|SetMinX (.X (Utilities|Struct|BreakIntVector4 _boundscount)))
  (LocalVariables|SetMaxX (.Y (Utilities|Struct|BreakIntVector4 _boundscount)))
  (LocalVariables|SetMinY (.Z (Utilities|Struct|BreakIntVector4 _boundscount)))
  (LocalVariables|SetMaxY (.W (Utilities|Struct|BreakIntVector4 _boundscount)))
  (Utilities|FlowControl|Sequence
    (:then_0
      ;[1 1 1] Main Loops
      (for _index (range (LocalVariables|GetMinY) (+ (LocalVariables|GetMaxY) -1))
        (LocalVariables|SetIndexY _index)
        (if bRandomRows
          (LocalVariables|SetVegIndex (Math|Random|RandomIntegerinRangefromStream (Math|Random|MakeRandomStream (* _index Seed)) 0 2)))
        (for _index_2 (range (LocalVariables|GetMinX) (+ (LocalVariables|GetMaxX) -1))
          (LocalVariables|SetIndexX _index_2)
          (LocalVariables|SetCurrentLocation (Math|Vector|MakeVector (.X (Math|Vector2D|BreakVector2D (+ (Class|KismetMathLibrary|GetRotated2D (Class|KismetMathLibrary|GetRotated2D (Math|Vector2D|MakeVector2D (* (LocalVariables|GetIndexX) _returnvalue) (* (LocalVariables|GetIndexY) _returnvalue)) (.Yaw (Math|Rotator|BreakRotator (Transformation|GetWorldRotation Spline)))) GridRotationAngle) (Math|Vector2D|MakeVector2D _x _y)))) (.Y (Math|Vector2D|BreakVector2D (+ (Class|KismetMathLibrary|GetRotated2D (Class|KismetMathLibrary|GetRotated2D (Math|Vector2D|MakeVector2D (* (LocalVariables|GetIndexX) _returnvalue) (* (LocalVariables|GetIndexY) _returnvalue)) (.Yaw (Math|Rotator|BreakRotator (Transformation|GetWorldRotation Spline)))) GridRotationAngle) (Math|Vector2D|MakeVector2D _x _y)))) 0.0))
          (LocalVariables|SetbInside (Math|Boolean|ANDBoolean (> (Math|Vector|DotProduct (Math|Vector|CrossProduct "0.000000,0.000000,1.000000" (Spline|FindDirectionClosesttoWorldLocation Spline (LocalVariables|GetCurrentLocation) "World")) (Math|Vector|Normalize (- (Spline|FindLocationClosesttoWorldLocation Spline (LocalVariables|GetCurrentLocation) "World") (LocalVariables|GetCurrentLocation)))) 0.0) (> (Math|Vector2D|Vector2DLength (- (Math|Vector2D|MakeVector2D (.X (Math|Vector|BreakVector (Spline|FindLocationClosesttoWorldLocation Spline (LocalVariables|GetCurrentLocation) "World"))) (.Y (Math|Vector|BreakVector (Spline|FindLocationClosesttoWorldLocation Spline (LocalVariables|GetCurrentLocation) "World")))) (Math|Vector2D|MakeVector2D (.X (Math|Vector|BreakVector (LocalVariables|GetCurrentLocation))) (.Y (Math|Vector|BreakVector (LocalVariables|GetCurrentLocation)))))) BorderPadding) (> (Math|Vector2D|Vector2DLength (- (Math|Vector2D|MakeVector2D (.X (Math|Vector|BreakVector (Spline|FindLocationClosesttoWorldLocation Path (LocalVariables|GetCurrentLocation) "World"))) (.Y (Math|Vector|BreakVector (Spline|FindLocationClosesttoWorldLocation Path (LocalVariables|GetCurrentLocation) "World")))) (Math|Vector2D|MakeVector2D (.X (Math|Vector|BreakVector (LocalVariables|GetCurrentLocation))) (.Y (Math|Vector|BreakVector (LocalVariables|GetCurrentLocation)))))) (* (.y (Class|SplineComponent|FindScaleClosesttoWorldLocation Path (LocalVariables|GetCurrentLocation))) PathSize))))
          (Math|Integer|IncrementInt (LocalVariables|GetCurrentPoint)
            (:%20%20
              (if (LocalVariables|GetbInside)
                (if bRandomRows
                  _
                  (else
                    (LocalVariables|SetVegIndex (Math|Random|RandomIntegerinRangefromStream (Math|Random|MakeRandomStream (* (LocalVariables|GetCurrentPoint) Seed)) 0 2))))
                (bind _returnvalue_3 (Utilities|Array|AddUnique _positions (LocalVariables|GetCurrentLocation)))
                (Utilities|Array|Resize _vegetables (Utilities|Array|Length _positions))
                (Utilities|Array|SetArrayElem _vegetables _returnvalue_3 (select bSinglePlantGarden OverrideVeggie (CallFunction|GetVeggie (LocalVariables|GetVegIndex))))))))))
    (:then_1
      (return (LocalVariables|GetPositions) (LocalVariables|GetVegetables)))))

(fn GetSplineBounds2D
  (params (Spline :type Spline%20Component%20Object%20Reference) (bWorldSpace :type Boolean) (Interval :type Float%20%28double-precision%29) (Padding :type Float%20%28double-precision%29))
  (bind _return (- Padding 0))
  (for _index (range 0 (- (Spline|GetNumberOfSplinePoints Spline) 1))
    (LocalVariables|SetXMin (Math|Float|Min(Float) (LocalVariables|GetXMin) (.x (Spline|GetLocationatSplinePoint Spline _index (select bWorldSpace "World" "Local")))))
    (LocalVariables|SetXMax (Math|Float|Max(Float) (LocalVariables|GetXMax) (.x (Spline|GetLocationatSplinePoint Spline _index (select bWorldSpace "World" "Local")))))
    (LocalVariables|SetYMin (Math|Float|Min(Float) (LocalVariables|GetYMin) (.y (Spline|GetLocationatSplinePoint Spline _index (select bWorldSpace "World" "Local")))))
    (LocalVariables|SetYMax (Math|Float|Max(Float) (LocalVariables|GetYMax) (.y (Spline|GetLocationatSplinePoint Spline _index (select bWorldSpace "World" "Local"))))))
  (return (Math|Vector4|MakeVector4 (LocalVariables|GetXMin) (LocalVariables|GetXMax) (LocalVariables|GetYMin) (LocalVariables|GetYMax)) (Utilities|Struct|MakeIntVector4 (Math|Float|Ceil (+ (/ (.X (Math|Vector4|BreakVector4 (Math|Vector4|MakeVector4 (LocalVariables|GetXMin) (LocalVariables|GetXMax) (LocalVariables|GetYMin) (LocalVariables|GetYMax)))) Interval) _return)) (Math|Float|Ceil (+ (/ (.Y (Math|Vector4|BreakVector4 (Math|Vector4|MakeVector4 (LocalVariables|GetXMin) (LocalVariables|GetXMax) (LocalVariables|GetYMin) (LocalVariables|GetYMax)))) Interval) Padding)) (Math|Float|Ceil (+ (/ (.Z (Math|Vector4|BreakVector4 (Math|Vector4|MakeVector4 (LocalVariables|GetXMin) (LocalVariables|GetXMax) (LocalVariables|GetYMin) (LocalVariables|GetYMax)))) Interval) _return)) (Math|Float|Ceil (+ (/ (.W (Math|Vector4|BreakVector4 (Math|Vector4|MakeVector4 (LocalVariables|GetXMin) (LocalVariables|GetXMax) (LocalVariables|GetYMin) (LocalVariables|GetYMax)))) Interval) Padding)))))

(fn GetVeggie
  (params (Index :type Integer))
  (return (Utilities|Select :Index Index :Option%200 (LocalVariables|GetCabbage) :Option%201 (LocalVariables|GetCorn) :Option%202 (LocalVariables|GetPumpkin))))