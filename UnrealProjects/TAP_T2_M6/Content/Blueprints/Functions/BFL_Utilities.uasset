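; Blueprint function library of small math helpers for negating a float and transforming a 2D vector by an angle.
; NegateFloat multiplies its input by -1.
; 2DRotate builds X and Y from dot products of the UV with (cos, sin) and (sin, cos) of the angle in degrees.
; Neither sine term is negated, so the result is not a true rotation, and a negated dot product sits unused.
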(fn NegateFloat
  (params (Value :type Float%20%28double-precision%29))
  (return (* Value -1.0)))

(fn 2DRotate
  (params (UV :type Vector%202D%20Structure) (RotationAngle :type Float%20%28double-precision%29))
  (bind _returnvalue (Math|Trig|Sin(Degrees) RotationAngle))
  (bind _returnvalue_2 (Math|Trig|Cos(Degrees) RotationAngle))
  (return (Math|Vector2D|MakeVector2D (Math|Vector2D|DotProduct(2D) UV (Math|Vector2D|MakeVector2D _returnvalue_2 _returnvalue)) (Math|Vector2D|DotProduct(2D) UV (Math|Vector2D|MakeVector2D _returnvalue _returnvalue_2)))))